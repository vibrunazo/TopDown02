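; Mob01 is a mob actor that handles its own death and awards the player a point for it.
; Each Tick checks the DestroyChar flag and, while it is set, destroys the Mesh component.
; A DoOnce then increases the MyGame game mode score by one, spawns an explosion emitter at the actor's location and destroys the actor after a short delay.
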(event `self.ReceiveTick`
  (params (DeltaSeconds :type "Float (single-precision)"))
  (if (`self.DestroyChar`)
    (`ActorComponent.K2_DestroyComponent` (`self.Mesh`))
    (`/Engine/EditorBlueprintResources/StandardMacros.DoOnce` false
      (:`Completed`
        (bind _asmy_game (cast `/Game/Blueprints/MyGame` (`GameplayStatics.GetGameMode`)))
        (`/Game/Blueprints/MyGame.IncreaseScore` _asmy_game 1)
        (`GameplayStatics.SpawnEmitterAtLocation` "/Game/StarterContent/Particles/P_Explosion.P_Explosion" (`self.K2_GetActorLocation`))
        (`KismetSystemLibrary.Delay` 5.0)
        (`self.K2_DestroyActor`)))))

(fn `UserConstructionScript`)
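; Projectile actor that explodes when it reaches ground level.
; Tick checks its height against a fixed Z threshold, then spawns a scaled-up KillZone at the impact point and destroys a component.
; A DoOnce guards only the explosion emitter and the briefly delayed actor destruction, so KillZone spawning repeats on each tick below the threshold until the actor is gone.
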(event `self.ReceiveTick`
  (params (DeltaSeconds :type "Float (single-precision)"))
  (bind _returnvalue (`self.K2_GetActorLocation`))
  (if (< (.z (`self.K2_GetActorLocation`)) 18.0)
    (`|SpawnActorFromClass` "/Game/Blueprints/KillZone.KillZone_C" (`KismetMathLibrary.MakeTransform` _returnvalue (struct) (5.0 5.0 5.0)) true)
    (`ActorComponent.K2_DestroyComponent`)
    (`/Engine/EditorBlueprintResources/StandardMacros.DoOnce` false
      (:`Completed`
        (`GameplayStatics.SpawnEmitterAtLocation` "/Game/StarterContent/Particles/P_Bigger_Explosion.P_Bigger_Explosion" (+ _returnvalue (0.0 0.0 100.0)))
        (`KismetSystemLibrary.Delay` 0.1)
        (`self.K2_DestroyActor`)))))

(fn `UserConstructionScript`)
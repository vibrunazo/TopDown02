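; Test Blueprint for sending web requests from keyboard input and printing the response.
; F builds a request with a test key/value pair, posts it to a URL variable and opens a Google link.
; G sends a GET to the same URL and binds a result event that prints the response's "message" field.
; A second result handler and a debug print are left unconnected.
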(event `Key|F`
  (:`Pressed`
    (bind _output_get (set `self.request` (`JsonFieldData.SetString` (`JsonFieldData.Create`) "testkey" "testvalue")))
    (`JsonFieldData.PostRequest` _output_get (`self.url_0`))
    (`KismetSystemLibrary.LaunchURL` "google.com")))

(event `CustomEvent_0`
  (`KismetSystemLibrary.PrintString` (`KismetStringLibrary.Conv_ObjectToString` (`self.request`))))

(event `Key|G`
  (:`Pressed`
    (bind _output_get (set `self.request` (`JsonFieldData.GetRequest` (`self.url_0`))))
    (add `JsonFieldData.OnGetResult` _output_get (delegate `onGetResult`))))

(event `onGetResult`
  (`KismetSystemLibrary.PrintString` (`JsonFieldData.GetString` (`self.request`) "message")))

(fn `UserConstructionScript`)
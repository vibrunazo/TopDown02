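; WaveController is an actor that endlessly spawns Wave actors at its own location to pace waves in the game.
; From BeginPlay it loops, calling CreateWave with one spawner and increasing both the Wave's Delay and the wait before the next as the Waves counter rises.
; CreateWave spawns the actor and then sets its Spawners and Delay.
; A disconnected, hand-timed sequence with escalating spawner counts remains unused.
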(event `self.ReceiveBeginPlay`
  (`self.createWave` 1 (+ (`KismetMathLibrary.Conv_IntToDouble` (`self.waves`)) 6.1) :!label _label)
  (set `self.waves` (+ (`self.waves`) 1))
  (`KismetSystemLibrary.Delay` (+ (* (`KismetMathLibrary.Conv_IntToDouble` (`self.waves`)) 2.15) 4.7))
  (goto _label))

(fn `createWave`
  (params (spawners :type Integer :default 0) (delay :type "Float (double-precision)" :default 0.0))
  (bind _returnvalue (`|SpawnActorFromClass` "/Game/Blueprints/wave.wave_C" (`KismetMathLibrary.MakeTransform` (`self.K2_GetActorLocation`))))
  (set `/Game/Blueprints/wave.spawners` spawners _returnvalue)
  (set `/Game/Blueprints/wave.delay` delay _returnvalue)
  (return))

(fn `UserConstructionScript`)
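; EndZone is an actor marking where Mob01 enemies cost the player a life.
; On overlap it destroys the Mob01, then calls DecreaseLife on the MyGame game mode while Lives remain above zero.
; Shortly after BeginPlay, it destroys itself unless its Permanent flag is set.
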(event `self.ReceiveActorBeginOverlap`
  (params (OtherActor :type "Actor Object Reference"))
  (bind _asmob_01 (cast `/Game/Blueprints/Mob01` OtherActor))
  (`self.K2_DestroyActor` _asmob_01)
  (bind _asmy_game (cast `/Game/Blueprints/MyGame` (`GameplayStatics.GetGameMode`)))
  (if (> (`/Game/Blueprints/MyGame.lives` _asmy_game) 0)
    (`/Game/Blueprints/MyGame.DecreaseLife` _asmy_game 1)))

(event `self.ReceiveBeginPlay`
  (`KismetSystemLibrary.Delay` 0.1)
  (if (not (`self.Permanent`))
    (`self.K2_DestroyActor`)))

(fn `UserConstructionScript`)
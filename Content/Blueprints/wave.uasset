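; Wave actor that randomizes the spawn timing of four Spawner child actors.
; On BeginPlay it casts each ChildActor component's actor to Spawner and sets its SpawnDelay to a random value, with the first and last spawners allowed a wider range than the middle two.
; The casts run in sequence, so one failed cast leaves the remaining spawners unconfigured.
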(event `self.ReceiveBeginPlay`
  (bind _asspawner (cast `/Game/Blueprints/Spawner` (`ChildActorComponent.ChildActor` (`self.ChildActor1`))))
  (set `/Game/Blueprints/Spawner.spawn delay` (`KismetMathLibrary.RandomFloatInRange` 1.0 3.0) _asspawner)
  (bind _asspawner_2 (cast `/Game/Blueprints/Spawner` (`ChildActorComponent.ChildActor` (`self.ChildActor2`))))
  (set `/Game/Blueprints/Spawner.spawn delay` (`KismetMathLibrary.RandomFloatInRange` 1.0 2.0) _asspawner_2)
  (bind _asspawner_3 (cast `/Game/Blueprints/Spawner` (`ChildActorComponent.ChildActor` (`self.ChildActor3`))))
  (set `/Game/Blueprints/Spawner.spawn delay` (`KismetMathLibrary.RandomFloatInRange` 1.0 2.0) _asspawner_3)
  (bind _asspawner_4 (cast `/Game/Blueprints/Spawner` (`ChildActorComponent.ChildActor` (`self.ChildActor4`))))
  (set `/Game/Blueprints/Spawner.spawn delay` (`KismetMathLibrary.RandomFloatInRange` 1.0 3.0) _asspawner_4))

(fn `UserConstructionScript`)
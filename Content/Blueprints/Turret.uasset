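; Turret actor that aims and shoots a Projectile at a supplied click location.
; Fire rotates StaticMesh2 to face the target, then spawns the projectile at that mesh's position with the same look-at rotation.
; Fire has no live caller in this Blueprint; Tick and the construction script are empty, and the delayed-spawn and test Fire chains are disconnected.
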(event `self.ReceiveTick`
  (params (DeltaSeconds :type "Float (single-precision)")))

(fn `Fire`
  (params (ClickLocation :type "Object.Vector Structure"))
  (bind _returnvalue (`SceneComponent.K2_GetComponentLocation` (`self.StaticMesh2`)))
  (bind _returnvalue_2 (`KismetMathLibrary.FindLookAtRotation` _returnvalue ClickLocation))
  (`SceneComponent.K2_SetWorldRotation` (`self.StaticMesh2`) _returnvalue_2 false)
  (`|SpawnActorFromClass` "/Game/Blueprints/Projectile.Projectile_C" (`KismetMathLibrary.MakeTransform` _returnvalue _returnvalue_2 (1.0 1.0 1.0))))

(fn `UserConstructionScript`)